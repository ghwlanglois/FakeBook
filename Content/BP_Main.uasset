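; Main controller for a political news-feed game that shows WBP_Main, adapts its articles daily and ends with WBP_EndScreen on day 5.
; ProcessImage turns likes and dislikes into clamped L/R scores using texture-name prefixes.
; ArticlesAlgorithm fills the feed from random left, right and post pools, weighting article mix by day and score.
; Branches contradict their comments, the all-left layout is unreachable, and removals re-roll the random index.
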(event Custom|ProcessImage
  (params (Image :type Texture%202D%20Object%20Reference) (Like? :type Boolean))
  (bind _returnvalue (Utilities|GetDisplayName Image))
  (bind _returnvalue_2 (Math|Integer|SelectInt 1 -1 Like?))
  (if (Utilities|String|Contains _returnvalue "LEFT_" true)
    (Variables|Default|SetL (Math|Integer|Clamp(Integer) (+ (Variables|Default|GetL) _returnvalue_2) 0 5))
    (elif (Utilities|String|Contains _returnvalue "RIGHT_" true)
      (Variables|Default|SetR (Math|Integer|Clamp(Integer) (+ _returnvalue_2 (Variables|Default|GetR)) 0 5)))))

(event Custom|NewDay
  (Math|Integer|IncrementInt (Variables|Default|GetDay)
    (:%20%20
      (CallFunction|ArticlesAlgorithm))))

(event EventBeginPlay
  ;[1 1 1] Add Main UI to screen
  (bind _returnvalue (UserInterface|CreateWidget "/Game/WBP_Main.WBP_Main_C"))
  (bind _output_get (Variables|Default|SetWBP_Main _returnvalue))
  (UserInterface|Viewport|AddtoViewport _output_get 1000)
  (CallFunction|ArticlesAlgorithm))

(fn ConstructionScript)

(fn ArticlesAlgorithm
  (bind _posts (Variables|Default|GetPosts))
  (bind _right_articles (Variables|Default|GetRight%20Articles))
  (bind _posts_2 (Variables|Default|GetPosts))
  (bind _left_articles (Variables|Default|GetLeft%20Articles))
  (bind _posts_3 (Variables|Default|GetPosts))
  (bind _right_articles_2 (Variables|Default|GetRight%20Articles))
  (bind _right_articles_3 (Variables|Default|GetRight%20Articles))
  (bind _l (Variables|Default|GetL))
  (bind _r (Variables|Default|GetR))
  (bind _posts_4 (Variables|Default|GetPosts))
  (bind _right_articles_4 (Variables|Default|GetRight%20Articles))
  (bind _right_articles_5 (Variables|Default|GetRight%20Articles))
  (bind _posts_5 (Variables|Default|GetPosts))
  (bind _right_articles_6 (Variables|Default|GetRight%20Articles))
  (bind _posts_6 (Variables|Default|GetPosts))
  (bind _right_articles_7 (Variables|Default|GetRight%20Articles))
  (bind _posts_7 (Variables|Default|GetPosts))
  (bind _posts_8 (Variables|Default|GetPosts))
  (bind _left_articles_2 (Variables|Default|GetLeft%20Articles))
  (bind _posts_9 (Variables|Default|GetPosts))
  (bind _right_articles_8 (Variables|Default|GetRight%20Articles))
  (bind _posts_10 (Variables|Default|GetPosts))
  (bind _left_articles_3 (Variables|Default|GetLeft%20Articles))
  (bind _right_articles_9 (Variables|Default|GetRight%20Articles))
  (bind _posts_11 (Variables|Default|GetPosts))
  (bind _left_articles_4 (Variables|Default|GetLeft%20Articles))
  (bind _left_articles_5 (Variables|Default|GetLeft%20Articles))
  (bind _posts_12 (Variables|Default|GetPosts))
  (bind _left_articles_6 (Variables|Default|GetLeft%20Articles))
  (bind _right_articles_10 (Variables|Default|GetRight%20Articles))
  (bind _returnvalue (Utilities|Array|Length _right_articles_4))
  (bind _returnvalue_2 (Utilities|Array|Length _posts_5))
  (bind _returnvalue_3 (Utilities|Array|Length _posts_4))
  (bind _returnvalue_4 (Utilities|Array|Length _right_articles_5))
  (bind _returnvalue_5 (Utilities|Array|Length _left_articles_4))
  (bind _returnvalue_6 (Utilities|Array|Length _posts_12))
  (bind _returnvalue_7 (Utilities|Array|Length _right_articles_9))
  (bind _returnvalue_8 (Utilities|Array|Length _right_articles_6))
  (bind _returnvalue_9 (Utilities|Array|Length _posts_7))
  (bind _returnvalue_10 (Utilities|Array|Length _right_articles_2))
  (bind _returnvalue_11 (Utilities|Array|Length _right_articles_3))
  (bind _returnvalue_12 (Utilities|Array|Length _posts_6))
  (bind _returnvalue_13 (Utilities|Array|Length _posts_8))
  (bind _returnvalue_14 (Utilities|Array|Length _right_articles_7))
  (bind _returnvalue_15 (Utilities|Array|Length _left_articles_2))
  (bind _returnvalue_16 (Utilities|Array|Length _posts_10))
  (bind _returnvalue_17 (Utilities|Array|Length _left_articles_5))
  (bind _returnvalue_18 (Utilities|Array|Length _left_articles_3))
  (bind _returnvalue_19 (Utilities|Array|Length _posts_9))
  (bind _returnvalue_20 (Utilities|Array|Length _posts_11))
  (bind _returnvalue_21 (Utilities|Array|Length _right_articles_8))
  (bind _returnvalue_22 (Utilities|Array|Length _left_articles_6))
  (bind _returnvalue_23 (Utilities|Array|Length _posts_2))
  (bind _returnvalue_24 (Utilities|Array|Length _right_articles_10))
  (bind _returnvalue_25 (Utilities|Array|Length _right_articles))
  (bind _returnvalue_26 (Utilities|Array|Length _posts))
  (bind _returnvalue_27 (Utilities|Array|Length _posts_3))
  (bind _returnvalue_28 (Utilities|Array|Length _left_articles))
  (bind _returnvalue_29 (- _returnvalue_16 1))
  (bind _returnvalue_30 (- _returnvalue_17 1))
  (bind _returnvalue_31 (- _returnvalue_18 1))
  (bind _returnvalue_32 (- _returnvalue_19 1))
  (bind _returnvalue_33 (- _returnvalue_20 1))
  (bind _returnvalue_34 (- _returnvalue_21 1))
  (bind _returnvalue_35 (- _returnvalue 1))
  (bind _returnvalue_36 (- _returnvalue_22 1))
  (bind _returnvalue_37 (- _returnvalue_23 1))
  (bind _returnvalue_38 (- _returnvalue_24 1))
  (bind _returnvalue_39 (- _returnvalue_25 1))
  (bind _returnvalue_40 (- _returnvalue_26 1))
  (bind _returnvalue_41 (- _returnvalue_27 1))
  (bind _returnvalue_42 (- _returnvalue_28 1))
  (bind _returnvalue_43 (- _returnvalue_2 1))
  (bind _returnvalue_44 (- _returnvalue_3 1))
  (bind _returnvalue_45 (- _returnvalue_4 1))
  (bind _returnvalue_46 (- _returnvalue_5 1))
  (bind _returnvalue_47 (- _returnvalue_8 1))
  (bind _returnvalue_48 (- _returnvalue_6 1))
  (bind _returnvalue_49 (- _returnvalue_9 1))
  (bind _returnvalue_50 (- _returnvalue_7 1))
  (bind _returnvalue_51 (- _returnvalue_10 1))
  (bind _returnvalue_52 (- _returnvalue_11 1))
  (bind _returnvalue_53 (- _returnvalue_12 1))
  (bind _returnvalue_54 (- _returnvalue_13 1))
  (bind _returnvalue_55 (- _returnvalue_14 1))
  (bind _returnvalue_56 (- _returnvalue_15 1))
  (bind _returnvalue_57 (Math|Random|RandomIntegerinRange 0 _returnvalue_29))
  (bind _returnvalue_58 (Math|Random|RandomIntegerinRange 0 _returnvalue_30))
  (bind _returnvalue_59 (Math|Random|RandomIntegerinRange 0 _returnvalue_31))
  (bind _returnvalue_60 (Math|Random|RandomIntegerinRange 0 _returnvalue_32))
  (bind _returnvalue_61 (Math|Random|RandomIntegerinRange 0 _returnvalue_33))
  (bind _returnvalue_62 (Math|Random|RandomIntegerinRange 0 _returnvalue_34))
  (bind _returnvalue_63 (Math|Random|RandomIntegerinRange 0 _returnvalue_35))
  (bind _returnvalue_64 (Math|Random|RandomIntegerinRange 0 _returnvalue_36))
  (bind _returnvalue_65 (Math|Random|RandomIntegerinRange 0 _returnvalue_37))
  (bind _returnvalue_66 (Math|Random|RandomIntegerinRange 0 _returnvalue_38))
  (bind _returnvalue_67 (Math|Random|RandomIntegerinRange 0 _returnvalue_39))
  (bind _returnvalue_68 (Math|Random|RandomIntegerinRange 0 _returnvalue_40))
  (bind _returnvalue_69 (Math|Random|RandomIntegerinRange 0 _returnvalue_41))
  (bind _returnvalue_70 (Math|Random|RandomIntegerinRange 0 _returnvalue_42))
  (bind _returnvalue_71 (Math|Random|RandomIntegerinRange 0 _returnvalue_43))
  (bind _returnvalue_72 (Math|Random|RandomIntegerinRange 0 _returnvalue_44))
  (bind _returnvalue_73 (Math|Random|RandomIntegerinRange 0 _returnvalue_45))
  (bind _returnvalue_74 (Math|Random|RandomIntegerinRange 0 _returnvalue_46))
  (bind _returnvalue_75 (Math|Random|RandomIntegerinRange 0 _returnvalue_47))
  (bind _returnvalue_76 (Math|Random|RandomIntegerinRange 0 _returnvalue_49))
  (bind _returnvalue_77 (Math|Random|RandomIntegerinRange 0 _returnvalue_48))
  (bind _returnvalue_78 (Math|Random|RandomIntegerinRange 0 _returnvalue_50))
  (bind _returnvalue_79 (Math|Random|RandomIntegerinRange 0 _returnvalue_51))
  (bind _returnvalue_80 (Math|Random|RandomIntegerinRange 0 _returnvalue_52))
  (bind _returnvalue_81 (Math|Random|RandomIntegerinRange 0 _returnvalue_53))
  (bind _returnvalue_82 (Math|Random|RandomIntegerinRange 0 _returnvalue_54))
  (bind _returnvalue_83 (Math|Random|RandomIntegerinRange 0 _returnvalue_55))
  (bind _returnvalue_84 (Math|Random|RandomIntegerinRange 0 _returnvalue_56))
  (bind _output (Utilities|Array|Get(acopy) _right_articles_4 _returnvalue_63))
  (bind _output_2 (Utilities|Array|Get(acopy) _left_articles_4 _returnvalue_74))
  (bind _output_3 (Utilities|Array|Get(acopy) _posts_12 _returnvalue_77))
  (bind _output_4 (Utilities|Array|Get(acopy) _right_articles_9 _returnvalue_78))
  (bind _output_5 (Utilities|Array|Get(acopy) _right_articles_6 _returnvalue_75))
  (bind _output_6 (Utilities|Array|Get(acopy) _posts_7 _returnvalue_76))
  (bind _output_7 (Utilities|Array|Get(acopy) _right_articles_2 _returnvalue_79))
  (bind _output_8 (Utilities|Array|Get(acopy) _right_articles_3 _returnvalue_80))
  (bind _output_9 (Utilities|Array|Get(acopy) _posts_6 _returnvalue_81))
  (bind _output_10 (Utilities|Array|Get(acopy) _posts_8 _returnvalue_82))
  (bind _output_11 (Utilities|Array|Get(acopy) _right_articles_7 _returnvalue_83))
  (bind _output_12 (Utilities|Array|Get(acopy) _left_articles_2 _returnvalue_84))
  (bind _output_13 (Utilities|Array|Get(acopy) _posts_10 _returnvalue_57))
  (bind _output_14 (Utilities|Array|Get(acopy) _left_articles_5 _returnvalue_58))
  (bind _output_15 (Utilities|Array|Get(acopy) _left_articles_3 _returnvalue_59))
  (bind _output_16 (Utilities|Array|Get(acopy) _posts_9 _returnvalue_60))
  (bind _output_17 (Utilities|Array|Get(acopy) _posts_11 _returnvalue_61))
  (bind _output_18 (Utilities|Array|Get(acopy) _right_articles_8 _returnvalue_62))
  (bind _output_19 (Utilities|Array|Get(acopy) _left_articles_6 _returnvalue_64))
  (bind _output_20 (Utilities|Array|Get(acopy) _posts_2 _returnvalue_65))
  (bind _output_21 (Utilities|Array|Get(acopy) _right_articles_10 _returnvalue_66))
  (bind _output_22 (Utilities|Array|Get(acopy) _right_articles _returnvalue_67))
  (bind _output_23 (Utilities|Array|Get(acopy) _posts _returnvalue_68))
  (bind _output_24 (Utilities|Array|Get(acopy) _posts_3 _returnvalue_69))
  (bind _output_25 (Utilities|Array|Get(acopy) _left_articles _returnvalue_70))
  (bind _output_26 (Utilities|Array|Get(acopy) _posts_5 _returnvalue_71))
  (bind _output_27 (Utilities|Array|Get(acopy) _posts_4 _returnvalue_72))
  (bind _output_28 (Utilities|Array|Get(acopy) _right_articles_5 _returnvalue_73))
  ;[1 1 1] check which day it is
  (LocalVariables|SetArticles (Utilities|Array|MakeArray (Variables|/Game/WBP_Main.WBP_Main_C|GetArticle0 (Variables|Default|GetWBP_Main)) (Variables|/Game/WBP_Main.WBP_Main_C|GetArticle1 (Variables|Default|GetWBP_Main)) (Variables|/Game/WBP_Main.WBP_Main_C|GetArticle2 (Variables|Default|GetWBP_Main)) (Variables|/Game/WBP_Main.WBP_Main_C|GetArticle3 (Variables|Default|GetWBP_Main))))
  (LocalVariables|SetAdsAndPosts (Utilities|Array|MakeArray (Variables|/Game/WBP_Main.WBP_Main_C|GetPost1 (Variables|Default|GetWBP_Main)) (Variables|/Game/WBP_Main.WBP_Main_C|GetPost2 (Variables|Default|GetWBP_Main)) (Variables|/Game/WBP_Main.WBP_Main_C|GetAd1 (Variables|Default|GetWBP_Main))))
  (switch int (Variables|Default|GetDay)
    (:1
      ;[1 1 1] Day 1 and L==R- 2 Lefty 2 Righty
      (Appearance|SetBrushfromTexture (Variables|/Game/WBP_Main.WBP_Main_C|GetArticle0 (Variables|Default|GetWBP_Main)) _output_19 false :!label _label)
      (Utilities|Array|RemoveItem _left_articles_6 _output_19)
      (Appearance|SetBrushfromTexture (Variables|/Game/WBP_Main.WBP_Main_C|GetPost1 (Variables|Default|GetWBP_Main)) _output_23 false)
      (Utilities|Array|RemoveItem _posts _output_23)
      (Appearance|SetBrushfromTexture (Variables|/Game/WBP_Main.WBP_Main_C|GetArticle1 (Variables|Default|GetWBP_Main)) _output_21 false)
      (Utilities|Array|RemoveItem _right_articles_10 _output_21)
      (Appearance|SetBrushfromTexture (Variables|/Game/WBP_Main.WBP_Main_C|GetAd1 (Variables|Default|GetWBP_Main)) _output_24 false)
      (Utilities|Array|RemoveItem _posts_3 _output_24)
      (Appearance|SetBrushfromTexture (Variables|/Game/WBP_Main.WBP_Main_C|GetArticle2 (Variables|Default|GetWBP_Main)) _output_25 false)
      (Utilities|Array|RemoveItem _left_articles _output_25)
      (Appearance|SetBrushfromTexture (Variables|/Game/WBP_Main.WBP_Main_C|GetPost2 (Variables|Default|GetWBP_Main)) _output_20 false)
      (Utilities|Array|RemoveItem _posts_2 _output_20)
      (Appearance|SetBrushfromTexture (Variables|/Game/WBP_Main.WBP_Main_C|GetArticle3 (Variables|Default|GetWBP_Main)) _output_22 false)
      (Utilities|Array|RemoveItem _right_articles _output_22))
    (:2
      ;[1 1 1] Day 2-4: Check if equal, if so do 1N, 2L, 2R
      (if (== _l _r) :!label _label_2
        (goto _label)
        (elif (== (Variables|Default|GetDay) 4)
          (if (> _l _r)
            ;[1 1 1] Day 2-3 - 3 Lefty 1 Righty
            (Appearance|SetBrushfromTexture (Variables|/Game/WBP_Main.WBP_Main_C|GetArticle0 (Variables|Default|GetWBP_Main)) _output_12 false)
            (Utilities|Array|RemoveItem _left_articles_2 _output_12)
            (Appearance|SetBrushfromTexture (Variables|/Game/WBP_Main.WBP_Main_C|GetPost1 (Variables|Default|GetWBP_Main)) _output_16 false)
            (Utilities|Array|RemoveItem _posts_9 _output_16)
            (Appearance|SetBrushfromTexture (Variables|/Game/WBP_Main.WBP_Main_C|GetArticle1 (Variables|Default|GetWBP_Main)) _output_14 false)
            (Utilities|Array|RemoveItem _left_articles_5 _output_14)
            (Appearance|SetBrushfromTexture (Variables|/Game/WBP_Main.WBP_Main_C|GetAd1 (Variables|Default|GetWBP_Main)) _output_17 false)
            (Utilities|Array|RemoveItem _posts_11 _output_17)
            (Appearance|SetBrushfromTexture (Variables|/Game/WBP_Main.WBP_Main_C|GetArticle2 (Variables|Default|GetWBP_Main)) _output_18 false)
            (Utilities|Array|RemoveItem _right_articles_8 _output_18)
            (Appearance|SetBrushfromTexture (Variables|/Game/WBP_Main.WBP_Main_C|GetPost2 (Variables|Default|GetWBP_Main)) _output_13 false)
            (Utilities|Array|RemoveItem _posts_10 _output_13)
            (Appearance|SetBrushfromTexture (Variables|/Game/WBP_Main.WBP_Main_C|GetArticle3 (Variables|Default|GetWBP_Main)) _output_15 false)
            (Utilities|Array|RemoveItem _left_articles_3 _output_15)
            (else
              ;[1 1 1] Day 2-3 - 3 Right 1 Lefty
              (Appearance|SetBrushfromTexture (Variables|/Game/WBP_Main.WBP_Main_C|GetArticle0 (Variables|Default|GetWBP_Main)) _output_4 false)
              (Utilities|Array|RemoveItem _right_articles_9 _output_4)
              (Appearance|SetBrushfromTexture (Variables|/Game/WBP_Main.WBP_Main_C|GetPost1 (Variables|Default|GetWBP_Main)) _output_3 false)
              (Utilities|Array|RemoveItem _posts_12 _output_3)
              (Appearance|SetBrushfromTexture (Variables|/Game/WBP_Main.WBP_Main_C|GetArticle1 (Variables|Default|GetWBP_Main)) _output_28 false)
              (Utilities|Array|RemoveItem _right_articles_5 _output_28)
              (Appearance|SetBrushfromTexture (Variables|/Game/WBP_Main.WBP_Main_C|GetAd1 (Variables|Default|GetWBP_Main)) _output_26 false)
              (Utilities|Array|RemoveItem _posts_5 _output_26)
              (Appearance|SetBrushfromTexture (Variables|/Game/WBP_Main.WBP_Main_C|GetArticle2 (Variables|Default|GetWBP_Main)) _output_2 false)
              (Utilities|Array|RemoveItem _left_articles_4 _output_2)
              (Appearance|SetBrushfromTexture (Variables|/Game/WBP_Main.WBP_Main_C|GetPost2 (Variables|Default|GetWBP_Main)) _output_27 false)
              (Utilities|Array|RemoveItem _posts_4 _output_27)
              (Appearance|SetBrushfromTexture (Variables|/Game/WBP_Main.WBP_Main_C|GetArticle3 (Variables|Default|GetWBP_Main)) _output false)
              (Utilities|Array|RemoveItem _right_articles_4 _output)))
          (elif (> _l _r)
            ;[1 1 1] Day 4- All Righty
            (Appearance|SetBrushfromTexture (Variables|/Game/WBP_Main.WBP_Main_C|GetArticle0 (Variables|Default|GetWBP_Main)) _output_5 false)
            (Utilities|Array|RemoveItem _right_articles_6 _output_5)
            (Appearance|SetBrushfromTexture (Variables|/Game/WBP_Main.WBP_Main_C|GetPost1 (Variables|Default|GetWBP_Main)) _output_9 false)
            (Utilities|Array|RemoveItem _posts_6 _output_9)
            (Appearance|SetBrushfromTexture (Variables|/Game/WBP_Main.WBP_Main_C|GetArticle1 (Variables|Default|GetWBP_Main)) _output_7 false)
            (Utilities|Array|RemoveItem _right_articles_2 _output_7)
            (Appearance|SetBrushfromTexture (Variables|/Game/WBP_Main.WBP_Main_C|GetAd1 (Variables|Default|GetWBP_Main)) _output_10 false)
            (Utilities|Array|RemoveItem _posts_8 _output_10)
            (Appearance|SetBrushfromTexture (Variables|/Game/WBP_Main.WBP_Main_C|GetArticle2 (Variables|Default|GetWBP_Main)) _output_11 false)
            (Utilities|Array|RemoveItem _right_articles_7 _output_11)
            (Appearance|SetBrushfromTexture (Variables|/Game/WBP_Main.WBP_Main_C|GetPost2 (Variables|Default|GetWBP_Main)) _output_6 false)
            (Utilities|Array|RemoveItem _posts_7 _output_6)
            (Appearance|SetBrushfromTexture (Variables|/Game/WBP_Main.WBP_Main_C|GetArticle3 (Variables|Default|GetWBP_Main)) _output_8 false)
            (Utilities|Array|RemoveItem _right_articles_3 _output_8)))))
    (:3
      (goto _label_2))
    (:4
      (goto _label_2))
    (:5
      ;[1 1 1] Day 5: Show the results
      (Widget|RemovefromParent (Variables|Default|GetWBP_Main))
      (Variables|Default|SetWBP_Main 0)
      (bind _returnvalue_85 (UserInterface|CreateWidget "/Game/WBP_EndScreen.WBP_EndScreen_C"))
      (bind _output_get (Variables|Default|SetWBP_EndScreen _returnvalue_85))
      (UserInterface|Viewport|AddtoViewport _output_get 10000))))

(fn SetArticle
  (params (image :type Image%20Object%20Reference) (LNRPA :type Integer))
  (bind _right_articles (Variables|Default|GetRight%20Articles))
  (bind _posts (Variables|Default|GetPosts))
  (bind _returnvalue (Utilities|Select :Index LNRPA :Option%200 0 :Option%201 0 :Option%202 _right_articles :Option%203 _posts :Option%204 0))
  (bind _returnvalue_2 (Utilities|Array|Length _returnvalue))
  (bind _returnvalue_3 (- _returnvalue_2 1))
  (bind _returnvalue_4 (Math|Random|RandomIntegerinRange 0 _returnvalue_3))
  (bind _output (Utilities|Array|Get(acopy) _returnvalue _returnvalue_4))
  (Appearance|SetBrushfromTexture image _output true)
  (Utilities|Array|RemoveItem _returnvalue _output))
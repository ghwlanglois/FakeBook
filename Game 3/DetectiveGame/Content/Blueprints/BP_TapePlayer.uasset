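; BP_TapePlayer is a tape player that plays a BP_Tape while one overlaps its Cylinder component.
; Each Tick polls the Cylinder's overlaps, and when no tape is current it calls PlayTape on the first one found and stores it as CurrentTape.
; The current tape holds the slot until no tapes overlap, then StopTape runs and the reference clears.
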(event EventBeginPlay
  (|CallParentFunction))

(event EventTick
  (params (DeltaSeconds :type Float%20%28single-precision%29))
  (bind _cylinder (Variables|Default|GetCylinder))
  (bind _overlappingactors (Collision|GetOverlappingActors _cylinder "/Game/Blueprints/BP_Tape.BP_Tape_C" :!class /Script/Engine.PrimitiveComponent))
  (bind _output (Utilities|Array|Get(acopy) _overlappingactors))
  (|CallParentFunction DeltaSeconds)
  (if (>= (Utilities|Array|Length _overlappingactors) 1)
    (Utilities|IsValid (Variables|Default|GetCurrentTape)
      (:Is%20Not%20Valid
        (Utilities|IsValid _output
          (:Is%20Valid
            (bind _asbp_tape (Utilities|Casting|CastToBP_Tape _output))
            (Default|PlayTape _asbp_tape)
            (Variables|Default|SetCurrentTape _asbp_tape)))))
    (else
      (Utilities|IsValid (Variables|Default|GetCurrentTape)
        (:Is%20Valid
          (Default|StopTape (Variables|Default|GetCurrentTape))
          (Variables|Default|SetCurrentTape 0))))))

(fn ConstructionScript
  (|CallParentFunction))
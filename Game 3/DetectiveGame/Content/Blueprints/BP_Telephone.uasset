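; BP_Telephone is a physics prop telephone that can be picked up and plays recorded calls when answered.
; RingPhone toggles the paused ring audio and sets the Ringing state, which is also applied on BeginPlay.
; Pickup disables physics and attaches the phone to a given component, and if ringing, stops the ring and plays the next recording from an indexed array.
; Drop restores physics and detaches it.
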(event Custom|RingPhone
  (params (True? :type Boolean))
  (Class|AudioComponent|SetPaused (Variables|Default|GetRingAudio) (not True?))
  (Variables|Default|SetRinging? True?))

(event Custom|PickUpPhone
  (bind _phonecallindex (Variables|Default|GetPhoneCallIndex))
  (bind _phoneaudio (Variables|Default|GetPhoneAudio))
  (CallFunction|RingPhone false)
  (Audio|Components|Audio|SetSound _phoneaudio (Utilities|Array|Get(acopy) (Variables|Default|GetAudioRecordings) _phonecallindex))
  (Audio|Components|Audio|Play _phoneaudio 0.0)
  (Math|Integer|IncrementInt _phonecallindex))

(event EventBeginPlay
  (CallFunction|RingPhone (Variables|Default|GetRinging?)))

(event Collision|EventActorBeginOverlap
  (params (OtherActor :type Actor%20Object%20Reference)))

(event EventTick
  (params (DeltaSeconds :type Float%20%28single-precision%29)))

(event EventPickup
  (params (AttachTo :type Scene%20Component%20Object%20Reference))
  (Physics|SetSimulatePhysics (Variables|Default|GetStaticMeshComponent) false)
  (Transformation|AttachComponentToComponent (VehicleSound|GetRootComponent) AttachTo "None" "KeepWorld" "KeepWorld" "KeepWorld" false)
  (if (Variables|Default|GetRinging?)
    (CallFunction|PickUpPhone)))

(event EventDrop
  (Physics|SetSimulatePhysics (Variables|Default|GetStaticMeshComponent) true)
  (Transformation|DetachFromActor "KeepWorld" "KeepWorld" "KeepWorld"))

(fn ConstructionScript)
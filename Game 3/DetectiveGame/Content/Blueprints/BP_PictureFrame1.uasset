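; Named picture frame for a clue puzzle, with face material and name text set at construction.
; Each tick it gathers pickup-interface actors overlapping its box and counts matches against the needed clue classes.
; Specific clue items load recordings onto a related phone and ring it, using flags to limit repeats.
; A full match reveals text and plays a sound, then rings the phone or, for "Tyler Thek", opens the "Fin" level.
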(event Custom|GetObjectsInBox
  (Utilities|Array|Clear (Variables|Default|GetActiveClues))
  (for _array_element (Collision|GetOverlappingActors (Variables|Default|GetBox) 0 :!class /Script/Engine.PrimitiveComponent)
    (if (Utilities|DoesObjectImplementInterface _array_element "/Game/VirtualRealityBP/Blueprints/PickupActorInterface.PickupActorInterface_C")
      (Utilities|Array|Add (Variables|Default|GetActiveClues) _array_element))))

(event Custom|CheckClues
  (bind _rolloftapeaudio (Variables|Default|GetRollOfTapeAudio))
  (bind _passage1audio (Variables|Default|GetPassage1Audio))
  (bind _relatedphone (Variables|Default|GetRelatedPhone))
  (bind _jacketaudio (Variables|Default|GetJacketAudio))
  (bind _keysaudio (Variables|Default|GetKeysAudio))
  (bind _boxcutteraudio (Variables|Default|GetBoxCutterAudio))
  (bind _output (Utilities|ResolveSoftReference _relatedphone))
  (Variables|Default|SetCluesNum 0)
  (for _array_element (Variables|Default|GetActiveClues)
    (for _array_element_2 (Variables|Default|GetNeededClues)
      (if (== _array_element_2 (Utilities|GetClass _array_element))
        (Math|Integer|IncrementInt (Variables|Default|GetCluesNum)
          (:%20%20
            _)))
      (Utilities|Casting|CastToBP_Jacket _array_element
        (:then
          (Variables|/Game/Blueprints/BP_Telephone.BP_Telephone_C|SetAudioRecordings _output _jacketaudio)
          (Utilities|IsValid _jacketaudio
            (:Is%20Valid
              (if (Variables|Default|GetJacketAudio_0)
                (Utilities|Casting|CastToBP_BoxCutter _array_element :!label _label
                  (:then
                    (Variables|/Game/Blueprints/BP_Telephone.BP_Telephone_C|SetAudioRecordings _output _boxcutteraudio)
                    (Utilities|IsValid _boxcutteraudio
                      (:Is%20Valid
                        (if (Variables|Default|GetBoxCutterAudio_0)
                          (Utilities|Casting|CastToBP_RollofTape _array_element :!label _label_2
                            (:then
                              (Variables|/Game/Blueprints/BP_Telephone.BP_Telephone_C|SetAudioRecordings _output _rolloftapeaudio)
                              (Utilities|IsValid _rolloftapeaudio
                                (:Is%20Valid
                                  (if (Variables|Default|GetRollOfTapeAudio_0)
                                    (Utilities|Casting|CastToBP_Keys _array_element :!label _label_3
                                      (:then
                                        (Variables|/Game/Blueprints/BP_Telephone.BP_Telephone_C|SetAudioRecordings _output _keysaudio)
                                        (Utilities|IsValid _keysaudio
                                          (:Is%20Valid
                                            (if (Variables|Default|GetKeysAudio_0)
                                              (Utilities|Casting|CastToGrateBP _array_element :!label _label_4)
                                              (Variables|/Game/Blueprints/BP_Telephone.BP_Telephone_C|SetAudioRecordings _output _passage1audio)
                                              (Utilities|IsValid _passage1audio
                                                (:Is%20Valid
                                                  (if (not (Variables|Default|GetPassage1Audio_0))
                                                    (Variables|Default|SetPassage1Audio_0 true)
                                                    (if (not false) :!label _label_5
                                                      (Default|RingPhone _output true)))))
                                              (else
                                                (Variables|Default|SetKeysAudio_0 true)
                                                (goto _label_5))))))
                                      (:CastFailed
                                        (goto _label_4)))
                                    (else
                                      (Variables|Default|SetRollOfTapeAudio_0 true)
                                      (goto _label_5))))))
                            (:CastFailed
                              (goto _label_3)))
                          (else
                            (Variables|Default|SetBoxCutterAudio_0 true)
                            (goto _label_5))))))
                  (:CastFailed
                    (goto _label_2)))
                (else
                  (Variables|Default|SetJacketAudio_0 true)
                  (goto _label_5))))))
        (:CastFailed
          (goto _label)))))
  (Rendering|SetVisibility (Variables|Default|GetTextRender) (== (Variables|Default|GetCluesNum) (Utilities|Array|Length (Variables|Default|GetNeededClues))) false)
  (if (== (Variables|Default|GetCluesNum) (Utilities|Array|Length (Variables|Default|GetNeededClues)))
    (Audio|PlaySound2D "/Game/Sounds/SoundEffects/TDSD_Found_a_Clue.TDSD_Found_a_Clue")
    (if (Utilities|Enum|Equal(Enum) (Variables|Default|GetName) (Utilities|Text|MakeLiteralText "Tyler Thek"))
      (Utilities|FlowControl|Delay 2.0)
      (Game|OpenLevel(byName) "Fin")
      (else
        (Default|RingPhone _output true)))))

(event EventBeginPlay
  (|CallParentFunction))

(event Collision|EventActorBeginOverlap
  (params (OtherActor :type Actor%20Object%20Reference))
  (|CallParentFunction OtherActor))

(event EventTick
  (params (DeltaSeconds :type Float%20%28single-precision%29))
  (|CallParentFunction DeltaSeconds)
  (Rendering|SetVisibility (Variables|Default|GetBox) (and (Physics|IsSimulatingPhysics (Variables|Debug|GetStaticMeshComponent) "None") (== (Math|Vector|VectorLength (Transformation|GetVelocity)) 0.0)) false)
  (CallFunction|GetObjectsinBox)
  (CallFunction|CheckClues))

(fn ConstructionScript
  (|CallParentFunction)
  (Rendering|Material|SetMaterial (Variables|Default|GetPainting) 0 (Variables|Default|GetFaceMaterial))
  (Rendering|Components|TextRender|SetText (Variables|Default|GetNameText) (Variables|Default|GetName)))
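; BP_Door is a door actor that swings open or closed when its Pickup or OpenClose event fires.
; BeginPlay stores the starting rotation, and a Rotate timeline adds its relative Z angle to that yaw on each update.
; OpenClose checks the Closed flag to play the matching 2D sound and run the timeline forward or in reverse.
; The flag flips only when the timeline finishes.
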(event Custom|OpenClose
  (bind _originalrotation (Variables|Default|GetOriginalRotation))
  (bind (_roll _pitch _yaw) (Math|Rotator|BreakRotator _originalrotation))
  (if (Variables|Default|GetClosed?)
    (Audio|PlaySound2D "/Game/Sounds/SoundEffects/TDSD_Door_Open.TDSD_Door_Open")
    (bind _relativezangle (Timeline|Rotate Play)
      (:Update
        (Transformation|SetActorRotation (Math|Rotator|MakeRotator _roll _pitch (+ _relativezangle _yaw))))
      (:Finished
        (Variables|Default|SetClosed? (not (Variables|Default|GetClosed?)))))
    (else
      (Audio|PlaySound2D "/Game/Sounds/SoundEffects/TDSD_Door_Close.TDSD_Door_Close")
      (Timeline|Rotate Reverse))))

(event EventBeginPlay
  (Variables|Default|SetOriginalRotation (Transformation|GetActorRotation)))

(event EventPickup
  (params (AttachTo :type Scene%20Component%20Object%20Reference))
  (CallFunction|OpenClose))

(fn ConstructionScript)
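; Tape actor that plays an assigned audio recording and visibly spins while it plays.
; PlayTape starts the recording from the beginning and uses a retriggerable delay matching its duration to call StopTape.
; StopTape pauses the audio and clears IsPlaying.
; While IsPlaying is set, Tick yaws both Cylinder and StaticMesh at a constant rate, based on the Cylinder's current rotation.
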(event Custom|PlayTape
  (bind _audiorecording (Variables|Default|GetAudioRecording))
  (bind _audio (Variables|Default|GetAudio))
  (Audio|Components|Audio|SetSound _audio _audiorecording)
  (Audio|Components|Audio|Play _audio 0.0)
  (Class|AudioComponent|SetPaused _audio false)
  (Variables|Default|SetIsPlaying? true)
  (Utilities|FlowControl|RetriggerableDelay (Variables|/Script/Engine.SoundBase|GetDuration _audiorecording))
  (CallFunction|StopTape))

(event Custom|StopTape
  (Class|AudioComponent|SetPaused (Variables|Default|GetAudio) true)
  (Variables|Default|SetIsPlaying? false))

(event EventBeginPlay
  (|CallParentFunction))

(event Collision|EventActorBeginOverlap
  (params (OtherActor :type Actor%20Object%20Reference))
  (|CallParentFunction OtherActor))

(event EventTick
  (params (DeltaSeconds :type Float%20%28single-precision%29))
  (bind _cylinder (Variables|Default|GetCylinder))
  (|CallParentFunction DeltaSeconds)
  (if (Variables|Default|GetIsPlaying?)
    (Transformation|SetRelativeRotation _cylinder (Math|Rotator|MakeRotator 0.0 0.0 (+ (.Yaw (Math|Rotator|BreakRotator (Variables|/Script/Engine.SceneComponent|GetRelativeRotation _cylinder))) (* DeltaSeconds 25.0))) false false)))

(fn ConstructionScript
  (|CallParentFunction))